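; Default arena character Blueprint that shows combat float text and a target indicator decal.
; An ability info delegate spawns a FloatTextWB for positive damage or healing caused by the local player, passing target, amount, heal and critical state.
; Tick shows the decal when the local player targets this character, matched by object name, with material chosen by team relationship.
; A debug sphere draw is left unconnected.
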(event `self.ReceiveBeginPlay`
  ;[1 1 1] Float Text
  (add `self.AbilityInfoDelegate` (delegate `OnAbilityInfoDelegate`)))

(event `OnAbilityInfoDelegate` :!signature `self.AbilityInfoDelegate`
  (params (AbilityInfo :type "AbilityInfo Structure"))
  (bind (_event _type _bisharmful _bisdispellable _bexpires _timeremaining _bcritical _amount _absorbed _overkill _causer _target) (break `AbilityInfo` AbilityInfo))
  ;[1 1 1] Float Text
  (if (and (== _causer (`GameplayStatics.GetPlayerCharacter` 0)) (> _amount 0.0))
    (switch `EAbilityInfoType` _type
      (:`EAIT_Damage`
        _)
      (:`EAIT_Heal`
        _))
    (bind _returnvalue (`|CreateWidget` "/Game/Widgets/Commons/FloatTextWB.FloatTextWB_C" (`GameplayStatics.GetPlayerController` 0)))
    (`/Engine/EditorBlueprintResources/StandardMacros.IsValid` _returnvalue
      (:`Is Valid`
        (`UserWidget.AddToViewport` _returnvalue 0)
        (`/Game/Widgets/Commons/FloatTextWB.Start` _returnvalue _target _amount (`|EnumEquality` _type "EAIT_Heal") (== _bcritical 1))))))

(event `self.ReceiveTick`
  (params (DeltaSeconds :type "Float (single-precision)"))
  (bind _decal (`self.Decal`))
  (bind _decal_2 (`self.Decal`))
  ;[1 1 1] Decal
  (bind _asarena_character (cast `ArenaCharacter` (`GameplayStatics.GetPlayerCharacter` 0)))
  (bind _target (`CharacterBase.Target` _asarena_character))
  (`/Engine/EditorBlueprintResources/StandardMacros.IsValid` _target
    (:`Is Valid`
      (if (`KismetStringLibrary.EqualEqual_StrStr` (`KismetSystemLibrary.GetObjectName` _target) (`KismetSystemLibrary.GetObjectName` self))
        (`SceneComponent.SetVisibility` _decal_2 true false)
        (bind _team (`CharacterBase.Team` _asarena_character))
        (switch `EPlayerTeam` _team
          (:`EPT_Red`
            (if (`|EnumEquality` (`self.Team`) _team) :!label _label
              (`DecalComponent.SetDecalMaterial` _decal "/Game/Materials/Target/ETargetDecalGreenMat.ETargetDecalGreenMat")
              (else
                (`DecalComponent.SetDecalMaterial` _decal "/Game/Materials/Target/ETargetDecalRedMat.ETargetDecalRedMat"))))
          (:`EPT_Blue`
            (goto _label))
          (:`EPT_Neutral`
            (`DecalComponent.SetDecalMaterial` _decal "/Game/Materials/Target/ETargetDecalNeutralMat.ETargetDecalNeutralMat")))
        (else
          (`SceneComponent.SetVisibility` _decal_2 false false :!label _label_2))))
    (:`Is Not Valid`
      (goto _label_2))))

(fn `UserConstructionScript`)