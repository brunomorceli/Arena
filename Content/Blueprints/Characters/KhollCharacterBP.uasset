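; Character Blueprint for Kholl that handles client-side targeting and combat feedback in the arena.
; Ability info events spawn floating damage or heal text when the local player is the causer.
; Tick shows a team-colored target decal when the player targets this character, and sets custom depth stencil by main-target and enemy status.
; Hovering the selection capsule switches the cursor by hostility; the player's own capsule has collision disabled.
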(event `self.ReceiveBeginPlay`
  ;[1 1 1] Float Text
  (add `ArenaCharacter.AbilityInfoDelegate` (delegate `OnAbilityInfoDelegate`))
  ;[1 1 1] Enable Mouse Cursor
  (bind _ascharacter_base (cast `CharacterBase` (`GameplayStatics.GetPlayerCharacter` 0)))
  (if (== _ascharacter_base self)
    (`PrimitiveComponent.SetCollisionEnabled` (`self.SelectionCapsule`) "NoCollision")))

(event `OnAbilityInfoDelegate`
  (params (AbilityInfo :type "AbilityInfo Structure"))
  (bind (_event _type _bisharmful _bisdispellable _bexpires _bdenied _timeremaining _stacks _bcritical _amount _absorbed _overkill _causer _target) (break `AbilityInfo` AbilityInfo))
  ;[1 1 1] Float Text
  (if (and (== _causer (`GameplayStatics.GetPlayerCharacter` 0)) (> _amount 0.0))
    (switch `EAbilityInfoType` _type
      (:`EAIT_Damage`
        _)
      (:`EAIT_Heal`
        _))
    (bind _returnvalue (`|CreateWidget` "/Game/Widgets/Commons/FloatTextWB.FloatTextWB_C" (`GameplayStatics.GetPlayerController` 0)))
    (`/Engine/EditorBlueprintResources/StandardMacros.IsValid` _returnvalue
      (:`Is Valid`
        (`UserWidget.AddToViewport` _returnvalue 0)
        (bind _asarena_character (cast `ArenaCharacter` _target))
        (`/Game/Widgets/Commons/FloatTextWB.Start` _returnvalue _asarena_character _amount (`|EnumEquality` _type "EAIT_Heal") (== _bcritical 1))))))

(event `self.ReceiveTick`
  (params (DeltaSeconds :type "Float (single-precision)"))
  (bind _decal (`self.Decal`))
  (bind _decal_2 (`self.Decal`))
  (bind _mesh (`self.Mesh`))
  (`|ExecutionSequence`
    (:`then_0`
      ;[1 1 1] Decal
      (bind _asarena_character (cast `ArenaCharacter` (`GameplayStatics.GetPlayerCharacter` 0)))
      (bind _target (`CharacterBase.Target` _asarena_character))
      (`/Engine/EditorBlueprintResources/StandardMacros.IsValid` _target
        (:`Is Valid`
          (if (`KismetStringLibrary.EqualEqual_StrStr` (`KismetSystemLibrary.GetObjectName` _target) (`KismetSystemLibrary.GetObjectName` self))
            (`SceneComponent.SetVisibility` _decal_2 true false)
            (bind _team (`CharacterBase.Team` _asarena_character))
            (switch `EPlayerTeam` _team
              (:`EPT_Red`
                (if (`|EnumEquality` (`self.Team`) _team) :!label _label
                  (`DecalComponent.SetDecalMaterial` _decal "/Game/Materials/Target/ETargetDecalGreenMat.ETargetDecalGreenMat")
                  (else
                    (`DecalComponent.SetDecalMaterial` _decal "/Game/Materials/Target/ETargetDecalRedMat.ETargetDecalRedMat"))))
              (:`EPT_Blue`
                (goto _label))
              (:`EPT_Neutral`
                (`DecalComponent.SetDecalMaterial` _decal "/Game/Materials/Target/ETargetDecalNeutralMat.ETargetDecalNeutralMat")))
            (else
              (`SceneComponent.SetVisibility` _decal_2 false false :!label _label_2))))
        (:`Is Not Valid`
          (goto _label_2))))
    (:`then_1`
      (bind _returnvalue (`self.IsMainTarget`))
      (if _returnvalue
        (bind _returnvalue_2 (`self.IsEnemy`))
        (if _returnvalue_2
          (`PrimitiveComponent.SetCustomDepthStencilValue` _mesh 2)
          (else
            (`PrimitiveComponent.SetCustomDepthStencilValue` _mesh 1)))
        (else
          (`PrimitiveComponent.SetCustomDepthStencilValue` _mesh 0))))))

(event `self.SelectionCapsule.OnBeginCursorOver`
  (params (TouchedComponent :type "PrimitiveComponent Object Reference"))
  (bind _returnvalue (`GameplayStatics.GetPlayerController` 0))
  ;[1 1 1] Mouse Over
  (bind _returnvalue_2 (`self.IsEnemy`))
  (if _returnvalue_2
    (set `PlayerController.CurrentMouseCursor` "Crosshairs" _returnvalue)
    (else
      (set `PlayerController.CurrentMouseCursor` "Hand" _returnvalue))))

(event `self.SelectionCapsule.OnEndCursorOver`
  (params (TouchedComponent :type "PrimitiveComponent Object Reference"))
  ;[1 1 1] Mouse Over
  (set `PlayerController.CurrentMouseCursor` "Default" (`GameplayStatics.GetPlayerController` 0)))

(fn `UserConstructionScript`)