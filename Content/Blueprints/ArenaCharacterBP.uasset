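; Arena character Blueprint that shows a target indicator decal when it is the first player character's current target.
; Every Tick it casts the player character to ArenaCharacter, compares its Target to itself by object name, and toggles the decal.
; For a Red or Blue player the decal is green on teammates and red otherwise, while a Neutral player gets the neutral material.
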(event `self.ReceiveTick`
  (params (DeltaSeconds :type "Float (single-precision)"))
  (bind _decal (`self.Decal`))
  (bind _decal_2 (`self.Decal`))
  ;[1 1 1] Decal
  (bind _asarena_character (cast `ArenaCharacter` (`GameplayStatics.GetPlayerCharacter` 0)))
  (bind _target (`CharacterBase.Target` _asarena_character))
  (`/Engine/EditorBlueprintResources/StandardMacros.IsValid` _target
    (:`Is Valid`
      (if (`KismetStringLibrary.EqualEqual_StrStr` (`KismetSystemLibrary.GetObjectName` _target) (`KismetSystemLibrary.GetObjectName` self))
        (`SceneComponent.SetVisibility` _decal_2 true false)
        (bind _team (`CharacterBase.Team` _asarena_character))
        (switch `EPlayerTeam` _team
          (:`EPT_Red`
            (if (`|EnumEquality` (`self.Team`) _team) :!label _label
              (`DecalComponent.SetDecalMaterial` _decal "/Game/Materials/Target/ETargetDecalGreenMat.ETargetDecalGreenMat")
              (else
                (`DecalComponent.SetDecalMaterial` _decal "/Game/Materials/Target/ETargetDecalRedMat.ETargetDecalRedMat"))))
          (:`EPT_Blue`
            (goto _label))
          (:`EPT_Neutral`
            (`DecalComponent.SetDecalMaterial` _decal "/Game/Materials/Target/ETargetDecalNeutralMat.ETargetDecalNeutralMat")))
        (else
          (`SceneComponent.SetVisibility` _decal_2 false false :!label _label_2))))
    (:`Is Not Valid`
      (goto _label_2))))

(fn `UserConstructionScript`)