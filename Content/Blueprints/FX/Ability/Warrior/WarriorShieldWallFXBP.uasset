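; Visual effect actor for the Warrior's Shield Wall ability, showing a spinning mesh on the character who owns it.
; On BeginPlay it casts its owner to ArenaCharacter and attaches to that character's pelvis socket.
; Each Tick rotates the mesh by a fixed step, independent of delta time, and polls the owner, destroying itself when the "Shield Wall - Physical Defense" ability entry is gone or the character dies.
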(event `self.ReceiveBeginPlay`
  (bind _asarena_character (cast `ArenaCharacter` (`self.GetOwner`)))
  (`/Engine/EditorBlueprintResources/StandardMacros.IsValid` _asarena_character
    (:`Is Valid`
      (set `self.ArenaCharacter` _asarena_character)
      (`self.K2_AttachToComponent` self (`Character.Mesh` _asarena_character) "pelvis_socket" "SnapToTarget" "KeepWorld" "KeepWorld" true))))

(event `self.ReceiveTick`
  (params (DeltaSeconds :type "Float (single-precision)"))
  (bind _arenacharacter (`self.ArenaCharacter`))
  (`SceneComponent.K2_AddRelativeRotation` (`self.StaticMesh`) (struct :`Yaw` 5.0) true true)
  (if (`.ReturnValue` (`BlueprintMapLibrary.Map_Find` (`CharacterBase.AbilityInfoList` _arenacharacter) "Shield Wall - Physical Defense"))
    (if (`|EnumEquality` (`CharacterBase.State` _arenacharacter) "CS_Death")
      (`self.K2_DestroyActor` :!label _label))
    (else
      (goto _label))))

(fn `UserConstructionScript`)