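; Temporary force wall effect that an ArenaCharacter owner can move through, built around a scaled Cube component.
; On BeginPlay it makes the owner's capsule ignore the Cube, then after a zero delay detaches to stay fixed in world space.
; One timeline animates the Cube's Y scale, and after a five-second hold a second timeline animates it again before the actor destroys itself.
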(event `self.ReceiveBeginPlay`
  (bind _cube (`self.Cube`))
  (bind _cube_2 (`self.Cube`))
  (bind _asarena_character (cast `ArenaCharacter` (`self.GetOwner`)))
  (`/Engine/EditorBlueprintResources/StandardMacros.IsValid` _asarena_character
    (:`Is Valid`
      (`PrimitiveComponent.IgnoreComponentWhenMoving` (`Character.CapsuleComponent` _asarena_character) _cube_2 true)
      (`KismetSystemLibrary.Delay` 0.0)
      (`self.K2_DetachFromActor` "KeepWorld" "KeepWorld" "KeepWorld")
      (bind (_direction _scale) (`Timeline|Timeline_0`)
        (:`Update`
          (`SceneComponent.SetWorldScale3D` _cube_2 (`KismetMathLibrary.MakeVector` (.x (`SceneComponent.K2_GetComponentScale` _cube_2)) _scale (.z (`SceneComponent.K2_GetComponentScale` _cube_2)))))
        (:`Finished`
          (`KismetSystemLibrary.Delay` 5.0)
          (bind (_direction_2 _scale_2) (`Timeline|Timeline_1`)
            (:`Update`
              (`SceneComponent.SetWorldScale3D` _cube (`KismetMathLibrary.MakeVector` (.x (`SceneComponent.K2_GetComponentScale` _cube)) _scale_2 (.z (`SceneComponent.K2_GetComponentScale` _cube)))))
            (:`Finished`
              (`self.K2_DestroyActor`))))))))

(fn `UserConstructionScript`)