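; Laser beam FX actor that shows a beam particle from its owning ArenaCharacter's right hand during a channel.
; After a short delay on BeginPlay, it attaches the beam emitter to the hand socket on the owner's mesh.
; Tick feeds the target's location into the beam's source tangent, rather than its target point.
; It destroys itself and the particle component when channelling stops or the target becomes invalid.
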(event `self.ReceiveBeginPlay`
  (`KismetSystemLibrary.Delay` 0.2)
  (bind _asarena_character (cast `ArenaCharacter` (`self.GetOwner`)))
  (`/Engine/EditorBlueprintResources/StandardMacros.IsValid` _asarena_character
    (:`Is Valid`
      (set `self.ArenaCharacter` _asarena_character)
      (bind _returnvalue (`GameplayStatics.SpawnEmitterAttached` "/Game/Particles/BeamAndLaserFX01/Particles/P_ky_beam01.P_ky_beam01" (`Character.Mesh` _asarena_character) "hand_r_socket"))
      (set `self.ParticleSystemComponent` _returnvalue))))

(event `self.ReceiveTick`
  (params (DeltaSeconds :type "Float (single-precision)"))
  (bind _arenacharacter (`self.ArenaCharacter`))
  (bind _particlesystemcomponent (`self.ParticleSystemComponent`))
  (bind _target (`CharacterBase.Target` _arenacharacter))
  (`/Engine/EditorBlueprintResources/StandardMacros.IsValid` _arenacharacter
    (:`Is Valid`
      (`/Engine/EditorBlueprintResources/StandardMacros.IsValid` (`self.ParticleSystemComponent`)
        (:`Is Valid`
          (if (`|EnumEquality` (`CharacterBase.AnimationState` _arenacharacter) "CAS_Channel")
            (`/Engine/EditorBlueprintResources/StandardMacros.IsValid` _target
              (:`Is Valid`
                (`ParticleSystemComponent.SetBeamSourceTangent` (`self.ParticleSystemComponent`) 0 (`self.K2_GetActorLocation` _target) 0))
              (:`Is Not Valid`
                (`self.K2_DestroyActor` :!label _label)
                (`/Engine/EditorBlueprintResources/StandardMacros.IsValid` _particlesystemcomponent
                  (:`Is Valid`
                    (`ActorComponent.K2_DestroyComponent` _particlesystemcomponent)))))
            (else
              (goto _label))))))))

(fn `UserConstructionScript`)