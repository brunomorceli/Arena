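; CastFXBP is an effect actor, named for casting, that follows the left hand of its owning CharacterBase.
; Every tick it casts its owner to CharacterBase and teleports itself to the mesh's hand_l_socket location, polling instead of attaching and leaving rotation untouched.
; It destroys itself once the owner's State is anything other than Idle.
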(event `self.ReceiveBeginPlay`)

(event `self.ReceiveTick`
  (params (DeltaSeconds :type "Float (single-precision)"))
  (bind _ascharacter_base (cast `CharacterBase` (`self.GetOwner`)))
  (`/Engine/EditorBlueprintResources/StandardMacros.IsValid` _ascharacter_base
    (:`Is Valid`
      (bind _mesh (`Character.Mesh` _ascharacter_base))
      (`self.K2_SetActorLocation` self (`SkeletalMeshSocket.GetSocketLocation` (`SkeletalMesh.FindSocket` (`SkinnedMeshComponent.SkeletalMesh` _mesh) "hand_l_socket") _mesh) false true)
      (if (`|EnumInequality` (`CharacterBase.State` _ascharacter_base) "CS_Idle")
        (`self.K2_DestroyActor`)))))

(fn `UserConstructionScript`)